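; Ground enemy Blueprint that drives death and base-attack animations for the Alien, Mutant and Zlorp enemy types.
; Both events find the mesh's anim instance type through a chain of casts to the three Animation Blueprints and set a flag on the match.
; EnemyDead sets IsDying, then destroys the actor after a short delay.
; StartAttackingBase sets AttackBase, with no other logic in this graph.
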(event EventStartAttackingBase
  (bind _mesh (Variables|Character|GetMesh))
  (bind _returnvalue (Components|SkeletalMesh|GetAnimInstance _mesh))
  (bind _asab_zlorp (Utilities|Casting|CastToAB_Zlorp _returnvalue)
    (:then
      (Variables|/Game/Enemies/Zlorp/AB_Zlorp.AB_Zlorp_C|SetAttackBase _asab_zlorp true))
    (:CastFailed
      (bind _asab_mutant (Utilities|Casting|CastToAB_Mutant _returnvalue)
        (:then
          (Variables|/Game/Enemies/Tank/AB_Mutant.AB_Mutant_C|SetAttackBase _asab_mutant true))
        (:CastFailed
          (bind _asab_alien (Utilities|Casting|CastToAB_Alien _returnvalue))
          (Variables|/Game/Enemies/Alien/AB_Alien.AB_Alien_C|SetAttackBase _asab_alien true))))))

(event EventEnemyDead
  (bind _mesh (Variables|Character|GetMesh))
  (bind _returnvalue (Components|SkeletalMesh|GetAnimInstance _mesh))
  (bind _asab_alien (Utilities|Casting|CastToAB_Alien _returnvalue)
    (:then
      (Variables|/Game/Enemies/Alien/AB_Alien.AB_Alien_C|SetIsDying _asab_alien true))
    (:CastFailed
      (bind _asab_mutant (Utilities|Casting|CastToAB_Mutant _returnvalue)
        (:then
          (Variables|/Game/Enemies/Tank/AB_Mutant.AB_Mutant_C|SetIsDying _asab_mutant true))
        (:CastFailed
          (bind _asab_zlorp (Utilities|Casting|CastToAB_Zlorp _returnvalue))
          (Variables|/Game/Enemies/Zlorp/AB_Zlorp.AB_Zlorp_C|SetIsDying _asab_zlorp true)))))
  (Utilities|FlowControl|Delay 2.0)
  (Actor|DestroyActor))

(fn ConstructionScript)